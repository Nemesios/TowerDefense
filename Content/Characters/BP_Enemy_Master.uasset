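; BP_Enemy_Master is an enemy that follows a spline path, takes damage and drops gold on death.
; Each Tick adds MovementSpeed to its spline distance without delta-time scaling, then moves it to that point, facing the direction of travel.
; AnyDamage reduces Life, and a lethal hit spawns BP_Pickup_Gold just above the actor before destroying it.
; The construction script sets the "Enemy" actor tag.
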(event Custom|Custom%20Drop%20Coin
  (Game|SpawnActorfromClass "/Game/Blueprints/BP_Pickup_Gold.BP_Pickup_Gold_C" (Math|Transform|MakeTransform (+ (Transformation|GetActorLocation) "0, 0,30.000000") "0,0.000000, 0" "1,1.000000,1") true 0))

(event EventTick
  (params (DeltaSeconds :type Float%20%28single-precision%29))
  (Variables|Default|SetDistance%20Along%20Spline (+ (Variables|Default|GetDistance%20Along%20Spline) (Variables|Default|GetMovement%20Speed)))
  (Transformation|SetWorldTransform (Math|Transform|MakeTransform (Class|SplineComponent|GetWorldLocationatDistanceAlongSpline (Variables|/Game/Blueprints/Spawner/Spline.Spline_C|GetSpline (Variables|Default|GetSpline_Blueprint)) (Variables|Default|GetDistance%20Along%20Spline)) (Math|Rotator|FindLookatRotation (Transformation|GetActorLocation) (Class|SplineComponent|GetWorldLocationatDistanceAlongSpline (Variables|/Game/Blueprints/Spawner/Spline.Spline_C|GetSpline (Variables|Default|GetSpline_Blueprint)) (Variables|Default|GetDistance%20Along%20Spline)))) false))

(event EventBeginPlay
  (Variables|Default|SetDistance%20Along%20Spline 0.0)
  (Transformation|SetWorldTransform (Math|Transform|MakeTransform (Class|SplineComponent|GetWorldLocationatDistanceAlongSpline (Variables|/Game/Blueprints/Spawner/Spline.Spline_C|GetSpline (Variables|Default|GetSpline_Blueprint)) (Variables|Default|GetDistance%20Along%20Spline)) (Math|Rotator|FindLookatRotation (Transformation|GetActorLocation) (Class|SplineComponent|GetWorldLocationatDistanceAlongSpline (Variables|/Game/Blueprints/Spawner/Spline.Spline_C|GetSpline (Variables|Default|GetSpline_Blueprint)) (Variables|Default|GetDistance%20Along%20Spline)))) false))

(event EventAnyDamage
  (params (Damage :type Float%20%28single-precision%29) (DamageType :type Damage%20Type%20Object%20Reference) (InstigatedBy :type Controller%20Object%20Reference) (DamageCauser :type Actor%20Object%20Reference))
  (if (<= (- (Variables|Default|GetLife) Damage) 0.0)
    (CallFunction|CustomDropCoin)
    (Actor|DestroyActor)
    (else
      (Variables|Default|SetLife (- (Variables|Default|GetLife) Damage)))))

(fn ConstructionScript
  (Variables|Default|SetTags (Utilities|Array|MakeArray "Enemy")))