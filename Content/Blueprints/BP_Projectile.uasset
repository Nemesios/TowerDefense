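; BP_Projectile is a homing projectile that chases a Target actor and damages it on contact.
; Each Tick moves the Projectile mesh toward the Target at Speed, scaled by delta time, and faces it using look-at rotation with pitch and yaw offsets.
; Overlapping the Target applies fixed damage and destroys the projectile, which also self-destructs when the Target becomes invalid.
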(event OnComponentBeginOverlap(Projectile)
  (params (OtherActor :type Actor%20Object%20Reference) (OtherComp :type Primitive%20Component%20Object%20Reference) (OtherBodyIndex :type Integer) (bFromSweep :type Boolean) (SweepResult :type Hit%20Result%20Structure%20%28by%20ref%29))
  (bind _target (Variables|Default|GetTarget))
  (if (== OtherActor _target)
    (Game|Damage|ApplyDamage _target 2.0 0 0)
    (Actor|DestroyActor)))

(event EventTick
  (params (DeltaSeconds :type Float%20%28single-precision%29))
  (bind _target (Variables|Default|GetTarget))
  (bind _projectile (Variables|Default|GetProjectile))
  (bind _returnvalue (Transformation|GetActorLocation _target))
  (bind _returnvalue_2 (Transformation|GetWorldLocation _projectile))
  (bind _returnvalue_3 (Math|Rotator|FindLookatRotation _returnvalue_2 _returnvalue))
  (bind (_pitch _yaw) (Class|KismetMathLibrary|BreakRot _returnvalue_3))
  ;[1 1 1] Set new location every frame
  (if (Utilities|IsValid (Variables|Default|GetTarget))
    (Transformation|SetWorldTransform (Variables|Default|GetProjectile) (Math|Transform|MakeTransform (+ (* (Math|Vector|Normalize (- (Transformation|GetActorLocation (Variables|Default|GetTarget)) (Transformation|GetWorldLocation (Variables|Default|GetProjectile)))) (* (Utilities|Time|GetWorldDeltaSeconds) (Variables|Default|GetSpeed))) (Transformation|GetWorldLocation (Variables|Default|GetProjectile))) (Class|KismetMathLibrary|MakeRot (+ _pitch -9e+01) (+ _yaw -9e+01) 0.0) "1,1.000000,1") false)
    (else
      (Actor|DestroyActor))))

(fn ConstructionScript
  (bind _returnvalue (AddComponent|AddStaticMeshComponent false))
  (Variables|Default|SetProjectile _returnvalue))