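; Player controller that owns the HUD and tracks the player's gold.
; On BeginPlay it creates the HUD widget, stores a reference and adds it to the viewport.
; A right click tells the HUD to hide its build menu.
; Increment and decrement functions adjust gold, clamped between zero and the maximum, and return the new total.
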(event EventBeginPlay
  (bind _returnvalue (UserInterface|CreateWidget "/Game/Blueprints/BP_Widget_HUD.BP_Widget_HUD_C" self))
  (Variables|Default|SetHUD%20Reference _returnvalue)
  (UserInterface|Viewport|AddtoViewport _returnvalue))

(event Input|ActionEvents|InputActionRightClick
  (:Pressed
    (Default|HideBuildMenu (Variables|Default|GetHUD%20Reference))))

(fn ConstructionScript)

(fn IncrementPlayerGold
  (params (ToAdd :type Integer))
  (Variables|Default|SetPlayerGold (Math|Integer|Clamp(Integer) (+ ToAdd (Variables|Default|GetPlayerGold)) 0 (Variables|Default|GetMaxGold)))
  (return (Variables|Default|GetPlayerGold)))

(fn DecrementPlayerGold
  (params (ToSub :type Integer))
  (Variables|Default|SetPlayerGold (Math|Integer|Clamp(Integer) (- (Variables|Default|GetPlayerGold) ToSub) 0 (Variables|Default|GetMaxGold)))
  (return (Variables|Default|GetPlayerGold)))