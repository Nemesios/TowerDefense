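; BP_Frost is a frost spell area that slows enemies while they stand inside it.
; When an actor tagged "enemy" enters the FrostArea overlap component, it is cast to BP_Enemy_Master and its MovementSpeed is halved.
; Leaving the area doubles the speed back, so the effect is a relative multiply rather than a stored original value.
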(event OnComponentBeginOverlap(FrostArea)
  (params (OtherActor :type Actor%20Object%20Reference) (OtherComp :type Primitive%20Component%20Object%20Reference) (OtherBodyIndex :type Integer) (bFromSweep :type Boolean) (SweepResult :type Hit%20Result%20Structure%20%28by%20ref%29))
  (if (Actor|ActorHasTag OtherActor "enemy")
    (bind _asbp_enemy_master (Utilities|Casting|CastToBP_Enemy_Master OtherActor))
    (Variables|/Game/Characters/BP_Enemy_Master.BP_Enemy_Master_C|SetMovement%20Speed _asbp_enemy_master (/ (Variables|/Game/Characters/BP_Enemy_Master.BP_Enemy_Master_C|GetMovement%20Speed _asbp_enemy_master) 2.0))))

(event OnComponentEndOverlap(FrostArea)
  (params (OtherActor :type Actor%20Object%20Reference) (OtherComp :type Primitive%20Component%20Object%20Reference) (OtherBodyIndex :type Integer))
  (if (Actor|ActorHasTag OtherActor "enemy")
    (bind _asbp_enemy_master (Utilities|Casting|CastToBP_Enemy_Master OtherActor))
    (Variables|/Game/Characters/BP_Enemy_Master.BP_Enemy_Master_C|SetMovement%20Speed _asbp_enemy_master (* (Variables|/Game/Characters/BP_Enemy_Master.BP_Enemy_Master_C|GetMovement%20Speed _asbp_enemy_master) 2.0))))

(fn ConstructionScript)