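; Level generator actor that builds a tile grid from a character-map string in its construction script.
; It fills a tile list pairing characters with grass and path tiles, then parses the string into rows of characters.
; Each cell switches on its character to add a child actor component as a tile.
; Tiles are offset by row and column index, with separate even and odd formulas centering the grid.
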(fn ConstructionScript
  (Utilities|FlowControl|Sequence
    (:then_0
      (|SetTilesList))
    (:then_1
      (|ParseString))
    (:then_2
      (|GetArraysLength))
    (:then_3
      (for (_array_element _array_index) (Variables|Default|GetMap)
        (for (_array_element_2 _array_index_2) (Utilities|Struct|BreakS_Map _array_element)
          (switch string _array_element_2
            (:0
              (bind _returnvalue (AddComponent|AddChildActorComponent false))
              (LocalVariables|SetNewChildActor _returnvalue))
            (:1
              (bind _returnvalue_2 (AddComponent|AddChildActorComponent false))
              (LocalVariables|SetNewChildActor _returnvalue_2))
            (:2
              (bind _returnvalue_3 (AddComponent|AddChildActorComponent false))
              (LocalVariables|SetNewChildActor _returnvalue_3)))
          (bind _result (CallFunction|ProcessOffsetTile (LocalVariables|GetSubArrayLength) _array_index_2))
          (bind _result_2 (CallFunction|ProcessOffsetTile (LocalVariables|GetArrayLength) _array_index))
          (Transformation|AddLocalOffset (LocalVariables|GetNewChildActor) (Math|Vector|MakeVector (Math|Conversions|ToFloat(Integer) _result) (Math|Conversions|ToFloat(Integer) _result_2) 0.0) false)
          (Class|SceneComponent|Attachto (LocalVariables|GetNewChildActor) 0 "None" "KeepRelativeOffset" true))))))

(fn ProcessOffsetTile
  (params (Length :type Integer) (Index :type Integer))
  (|IsEvenOrOdd Length
    (:IsEven
      (LocalVariables|SetOffset (|CalcEven Length Index)))
    (:IsOdd
      (LocalVariables|SetOffset (|CalcOdd Length Index))))
  (return (LocalVariables|GetOffset)))