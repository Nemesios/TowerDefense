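; BP_Tower is a tower that tracks targets inside its Tower_Attack_Area component.
; Overlapping actors other than BP_Projectile and BP_Cannon_Ball join TargetArray and set IsInRange, with a lone entry becoming Target.
; When any tracked actor leaves, Target switches to the entry that slides into its slot.
; If that slot is invalid, IsInRange clears even if earlier entries remain; no firing logic is present.
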(event OnComponentBeginOverlap(Tower_Attack_Area)
  (params (OtherActor :type Actor%20Object%20Reference) (OtherComp :type Primitive%20Component%20Object%20Reference) (OtherBodyIndex :type Integer) (bFromSweep :type Boolean) (SweepResult :type Hit%20Result%20Structure%20%28by%20ref%29))
  (Utilities|Casting|CastToBP_Projectile OtherActor
    (:CastFailed
      (Utilities|Casting|CastToBP_Cannon_Ball OtherActor
        (:CastFailed
          (Utilities|Array|Add (Variables|Default|GetTarget_Array) OtherActor)
          (Variables|Default|SetisInRange true)
          (Math|Integer|CompareInt (Utilities|Array|Length (Variables|Default|GetTarget_Array)) 1
            (:==
              (Variables|Default|SetTarget OtherActor))))))))

(event OnComponentEndOverlap(Tower_Attack_Area)
  (params (OtherActor :type Actor%20Object%20Reference) (OtherComp :type Primitive%20Component%20Object%20Reference) (OtherBodyIndex :type Integer))
  (bind _target_array (Variables|Default|GetTarget_Array))
  (for _index (range 0 (Utilities|Array|Length (Variables|Default|GetTarget_Array)))
    (if (== (Utilities|Array|Get(acopy) _target_array _index) OtherActor)
      (Utilities|Array|RemoveItem _target_array (Utilities|Array|Get(acopy) _target_array _index))
      (if (Utilities|IsValid (Utilities|Array|Get(acopy) _target_array _index))
        (Variables|Default|SetTarget (Utilities|Array|Get(acopy) _target_array _index))
        (else
          (Variables|Default|SetisInRange false))))))

(fn ConstructionScript)