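; BP_Pickup_Master is a base pickup actor with a configurable mesh, scale and material appearance.
; The construction script applies these settings and creates a dynamic material instance to set color and phase parameters.
; On BeginPlay, a looping timer spins the mesh when rotation is enabled, while the hover branch is empty.
; EndBehavior simply destroys the actor and has no caller in this graph.
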(event EventBeginPlay
  (Utilities|FlowControl|Sequence
    (:then_0
      (if (Variables|Default|GetIsRotating)
        (Utilities|Time|SetTimerbyFunctionName self "Rotate" (Variables|Default|GetRotationTimer) true)))
    (:then_1
      (if (Variables|Default|GetIsHovering)
        _))))

(fn ConstructionScript
  (Rendering|Material|SetMaterial 0 (Variables|Default|GetCoreMaterial))
  (bind _returnvalue (Rendering|Material|CreateDynamicMaterialInstance (Variables|Default|GetPickupMesh) 0 (Variables|Default|GetCoreMaterial) :!class /Script/Engine.PrimitiveComponent))
  (Variables|Default|SetMaterialInst _returnvalue)
  (Components|StaticMesh|SetStaticMesh (Variables|Default|GetMesh))
  (Transformation|SetRelativeScale3D (Variables|Default|GetPickupMesh) (Variables|Default|GetScale))
  (Rendering|Material|SetVectorParameterValue (Variables|Default|GetMaterialInst) "Color" (Variables|Default|GetColor) :!class /Script/Engine.MaterialInstanceDynamic)
  (Rendering|Material|SetScalarParameterValue (Variables|Default|GetMaterialInst) "Phase" (Variables|Default|GetPhase) :!class /Script/Engine.MaterialInstanceDynamic))

(fn EndBehavior
  (Actor|DestroyActor))

(fn Rotate
  (Transformation|AddLocalRotation (Variables|Default|GetPickupMesh) (Variables|Default|GetRotationRate) false))