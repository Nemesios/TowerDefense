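; BP_Tile_Grass is a clickable grass tile that serves as a tower build slot.
; Hovering swaps its material to a highlight and toggles a visibility cue, while construction shows or hides the Grid from ShowGrid.
; Clicking registers it as the player controller's FocusTile and opens the HUD's build menu, or the upgrade menu if occupied.
; CustomSpawnTower spawns the given class at SocketTower and marks the tile occupied.
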(event Custom|Custom%20SpawnTower
  (params (NewParam :type BP%20Tower%20Class%20Reference))
  (bind _returnvalue (Game|SpawnActorfromClass NewParam (Math|Transform|MakeTransform (Transformation|GetWorldLocation (Variables|Default|GetSocketTower)) "0,0.000000, 0" "1.000000,1,1") false 0))
  (Variables|Default|SetTower _returnvalue)
  (Variables|Default|SetHasTower true))

(event EventActorOnClicked
  (bind _playercontroller (Variables|Default|GetPlayerController))
  (bind _hud_reference (Variables|/Game/Blueprints/BP_Mouse_PlayerController.BP_Mouse_PlayerController_C|GetHUD%20Reference _playercontroller))
  (Variables|/Game/Blueprints/BP_Mouse_PlayerController.BP_Mouse_PlayerController_C|SetFocusTile (Variables|Default|GetPlayerController) self)
  (if (Variables|Default|GetHasTower)
    (Default|DisplayUpgradeMenu _hud_reference (Variables|Default|GetTower))
    (else
      (Default|DisplayBuildMenu _hud_reference))))

(event EventBeginPlay
  (bind _asbp_mouse_player_controller (Utilities|Casting|CastToBP_Mouse_PlayerController (Game|GetPlayerController 0)))
  (Variables|Default|SetPlayerController _asbp_mouse_player_controller))

(event EventActorBeginCursorOver
  (Rendering|Material|SetMaterial 0 (Variables|Default|GetMaterialHighlight))
  (Rendering|SetVisibility true false))

(event EventActorEndCursorOver
  (Rendering|Material|SetMaterial 0 (Variables|Default|GetMaterialTile))
  (Rendering|SetVisibility false false))

(fn ConstructionScript
  (bind _grid (Variables|Default|GetGrid))
  (|CallParentFunction)
  (if (Variables|Default|GetShowGrid)
    (Rendering|SetVisibility _grid true true)
    (else
      (Rendering|SetVisibility _grid false true))))