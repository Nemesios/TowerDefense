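; Level generator Blueprint that builds a tile grid from a character map string in its Construction Script.
; The string is parsed into rows of characters, and each character (0–3, S, E or default) selects a branch that adds a child actor component.
; Even/odd offset math centres the grid on the actor, using the first row's length as width.
; A tile lookup list is also filled, but spawning does not read it.
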(fn ConstructionScript
  (bind _newchildactor (LocalVariables|GetNewChildActor))
  (Utilities|FlowControl|Sequence
    (:then_0
      (|SetTilesList))
    (:then_1
      (|ParseString))
    (:then_2
      (|GetArraysLength))
    (:then_3
      (for (_array_element _array_index) (Variables|Default|GetMap)
        (for (_array_element_2 _array_index_2) (Utilities|Struct|BreakS_Map _array_element)
          (switch string _array_element_2
            (:Default
              (goto _label Default))
            (:0
              (|AddChildActor :!label _label
                (:then0
                  _)
                (:then1
                  _)
                (:then2
                  _)
                (:then3
                  _)
                (:thens
                  _)
                (:thene
                  _)
                (:thenDefault
                  _))
              (bind _result (CallFunction|ProcessOffsetTile (LocalVariables|GetSubArrayLength) _array_index_2))
              (bind _result_2 (CallFunction|ProcessOffsetTile (LocalVariables|GetArrayLength) _array_index))
              (Transformation|AddLocalOffset _newchildactor (Math|Vector|MakeVector (Math|Conversions|ToFloat(Integer) _result) (Math|Conversions|ToFloat(Integer) _result_2) 0.0) false)
              (Class|SceneComponent|Attachto _newchildactor 0 "None" "KeepRelativeOffset" true))
            (:1
              (goto _label 1))
            (:2
              (goto _label 2))
            (:3
              (goto _label 3))
            (:s
              (goto _label s))
            (:e
              (goto _label e))))))))

(fn ProcessOffsetTile
  (params (Length :type Integer) (Index :type Integer))
  (|IsEvenOrOdd Length
    (:IsEven
      (LocalVariables|SetOffset (|CalcEven Length Index)))
    (:IsOdd
      (LocalVariables|SetOffset (|CalcOdd Length Index))))
  (return (LocalVariables|GetOffset)))