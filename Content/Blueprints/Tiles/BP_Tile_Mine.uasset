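; BP_Tile_Mine is a mine tile that periodically shows a gold rock the player clicks to collect gold.
; BeginPlay caches the mouse player controller and starts a looping timer, its interval randomized once, that reveals the Mine component if hidden.
; Clicking a revealed rock hides it, spawns an explosion particle above SocketParticle and adds Value to the player's gold through the controller.
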(event Custom|Spawn%20Gold%20Rock
  (if (not (Variables|Default|GetGoldRockSpawned))
    (Rendering|SetVisibility (Variables|Default|GetMine) true false)
    (Variables|Default|SetGoldRockSpawned true)))

(event EventBeginPlay
  (bind _asbp_mouse_player_controller (Utilities|Casting|CastToBP_Mouse_PlayerController (Game|GetPlayerController 0)))
  (Variables|Default|SetPlayerController _asbp_mouse_player_controller)
  (Utilities|Time|SetTimerbyFunctionName self "Spawn Gold Rock" (Math|Conversions|ToFloat(Integer) (Math|Random|RandomInteger (Variables|Default|GetmaxTimer))) true))

(event EventActorOnClicked
  (if (Variables|Default|GetGoldRockSpawned)
    (Rendering|SetVisibility (Variables|Default|GetMine) false false)
    (Variables|Default|SetGoldRockSpawned false)
    (Effects|SpawnEmitteratLocation "/Game/Particles/P_Explosion.P_Explosion" (+ (Transformation|GetWorldLocation (Variables|Default|GetSocketParticle)) "0, 0,50.000000") "0,0.000000, 0")
    (Default|CustomeIncrementPlayerGold (Variables|Default|GetPlayerController) (Variables|Default|GetValue))))

(fn ConstructionScript
  (|CallParentFunction))