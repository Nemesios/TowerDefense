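; Spawner actor that spawns a queued number of enemies of a selected type, with a helper that queues five Goblins when none remain.
; Spawn sets the enemy type, adds to the remaining count and toggles the spawning flag.
; While active, Tick uses a Delay to space spawns, counts down, and toggles off at zero.
; Each enemy appears at the actor's location offset by its right vector, facing its forward direction.
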(event EventTick
  (params (DeltaSeconds :type Float%20%28single-precision%29))
  (if (and (Variables|Default|GetisSpawning) (> (Variables|Default|GetNumber%20To%20Spawn) 0))
    (Utilities|FlowControl|Delay (Variables|Default|GetSpawning%20Speed))
    (CallFunction|SpawnEnemy)
    (Variables|Default|SetNumber%20To%20Spawn (- (Variables|Default|GetNumber%20To%20Spawn) 1))
    (if (and (<= (Variables|Default|GetNumber%20To%20Spawn) 0) (Variables|Default|GetisSpawning))
      (CallFunction|SwitchMode))))

(fn ConstructionScript)

(fn SpawnEnemy
  (Game|SpawnActorfromClass (Variables|Default|GetEnemy%20Type) (Math|Transform|MakeTransform (Math|Transform|TransformLocation (Math|Transform|MakeTransform (Transformation|GetActorRightVector)) (Transformation|GetActorLocation)) (Math|Conversions|RotationFromXVector (Transformation|GetActorForwardVector)) "1.000000,1,1") false 0))

(fn SwitchMode
  (if (Variables|Default|GetisSpawning)
    (Variables|Default|SetisSpawning false)
    (else
      (Variables|Default|SetisSpawning true))))

(fn SelectEnemy
  (params (Enemy%20type :type Enemy%20Class%20Reference))
  (Variables|Default|SetEnemy%20Type Enemy%20type))

(fn Spawn
  (params (Enemy%20type :type Enemy%20Class%20Reference) (Number%20of%20Enemy :type Integer))
  (CallFunction|SelectEnemy Enemy%20type)
  (Variables|Default|SetNumber%20To%20Spawn (+ (Variables|Default|GetNumber%20To%20Spawn) Number%20of%20Enemy))
  (CallFunction|SwitchMode))

(fn Spawn5Gob
  (if (<= (Variables|Default|GetNumber%20To%20Spawn) 0)
    (CallFunction|Spawn "/Game/Characters/Goblin.Goblin_C" 5)))