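; Cannon tower, a child tower Blueprint that turns its cannon toward a target in range and fires cannonballs at it.
; Each tick it rotates the cannon on yaw only; TowerShoot spawns a BP_Cannon_Ball, passes it target and damage, and plays a shot sound.
; LevelUp shortens reload, raises damage, plays effects and swaps in stone tower meshes by level.
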(event EventTick
  (params (DeltaSeconds :type Float%20%28single-precision%29))
  (bind (_returnvalue _cannon) (|RotateTowardTarget))
  (if (Variables|Default|GetisInRange)
    (Transformation|SetWorldRotation _cannon _returnvalue false)))

(event EventLevelUp
  (CallFunction|LevelUpCannon))

(event EventTowerShoot
  (CallFunction|CannonShoot))

(fn ConstructionScript
  (|CallParentFunction)
  (Variables|Default|SetProjectile "/Game/Blueprints/Tower/BP_Cannon_Ball.BP_Cannon_Ball_C"))

(fn CannonShoot
  (bind _returnvalue (Game|SpawnActorfromClass (Variables|Default|GetProjectile) (|SpawnLocation) false 0))
  (bind _asbp_cannon_ball (Utilities|Casting|CastToBP_Cannon_Ball _returnvalue))
  (Variables|/Game/Blueprints/Tower/BP_Cannon_Ball.BP_Cannon_Ball_C|SetTarget _asbp_cannon_ball (Variables|Default|GetTarget))
  (Variables|/Game/Blueprints/Tower/BP_Cannon_Ball.BP_Cannon_Ball_C|SetDamage _asbp_cannon_ball (Variables|Default|GetProjectileDamage))
  (Audio|PlaySoundatLocation "/Game/Sound/S_CannonShot.S_CannonShot" (Transformation|GetActorLocation _returnvalue)))

(fn LevelUpCannon
  (bind _tower_attack_area (Variables|Default|GetTower_Attack_Area))
  (bind _returnvalue (Transformation|GetWorldLocation _tower_attack_area))
  (Variables|Default|SetReloadTime (- (Variables|Default|GetReloadTime) 0.25))
  (Variables|Default|SetProjectileDamage (+ (Variables|Default|GetProjectileDamage) 2.0))
  (Variables|Default|SetLevel (+ (Variables|Default|GetLevel) 1))
  (Effects|SpawnEmitteratLocation "/Game/Particles/P_LevelUp.P_LevelUp" _returnvalue)
  (Audio|PlaySoundatLocation "/Game/Sound/S_LevelUp.S_LevelUp" _returnvalue)
  (if (== (Variables|Default|GetLevel) 1)
    (Components|StaticMesh|SetStaticMesh (Variables|Default|GettowerBase) "/Game/Meshes/StoneTower.StoneTower")
    (else
      (Components|StaticMesh|SetStaticMesh "/Game/Meshes/ProtectedStoneTower.ProtectedStoneTower"))))