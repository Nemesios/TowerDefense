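; Tower actor for a tower-defense game that tracks enemies in range and opens an upgrade menu when clicked.
; Overlaps on Tower_Attack_Area maintain an array of "Enemy"-tagged actors, setting the first as Target and choosing a replacement on exit.
; A looping TowerShoot timer runs at ReloadTime until no replacement is found.
; TowerShoot and LevelUp are empty here; clicks pass the tower to the player controller's HUD.
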(event OnComponentBeginOverlap(Tower_Attack_Area)
  (params (OtherActor :type Actor%20Object%20Reference) (OtherComp :type Primitive%20Component%20Object%20Reference) (OtherBodyIndex :type Integer) (bFromSweep :type Boolean) (SweepResult :type Hit%20Result%20Structure%20%28by%20ref%29))
  (if (Actor|ActorHasTag OtherActor (Utilities|String|StringToName "Enemy"))
    (Utilities|Array|Add (Variables|Default|GetTarget_Array) OtherActor)
    (Variables|Default|SetisInRange true)
    (Math|Integer|CompareInt (Utilities|Array|Length (Variables|Default|GetTarget_Array)) 1
      (:==
        (Variables|Default|SetTarget OtherActor)
        (CallFunction|TargetinRange)))))

(event OnComponentEndOverlap(Tower_Attack_Area)
  (params (OtherActor :type Actor%20Object%20Reference) (OtherComp :type Primitive%20Component%20Object%20Reference) (OtherBodyIndex :type Integer))
  (bind _target_array (Variables|Default|GetTarget_Array))
  (for _index (range 0 (Utilities|Array|Length (Variables|Default|GetTarget_Array)))
    (if (== (Utilities|Array|Get(acopy) _target_array _index) OtherActor)
      (Utilities|Array|RemoveItem _target_array (Utilities|Array|Get(acopy) _target_array _index))
      (if (Utilities|IsValid (Utilities|Array|Get(acopy) _target_array _index))
        (Variables|Default|SetTarget (Utilities|Array|Get(acopy) _target_array _index))
        (else
          (Variables|Default|SetisInRange false)
          (CallFunction|TargetNotinRange))))))

(event Custom|TargetInRange
  (Utilities|Time|SetTimerbyFunctionName 0 "TowerShoot" (Variables|Default|GetReloadTime) true))

(event Custom|TargetNotInRange
  (Utilities|Time|ClearTimerbyFunctionName 0 "TowerShoot"))

(event EventActorOnClicked
  (bind _asbp_mouse_player_controller (Utilities|Casting|CastToBP_Mouse_PlayerController (Game|GetPlayerController 0)))
  (Default|DisplayUpgradeMenu (Variables|/Game/Blueprints/BP_Mouse_PlayerController.BP_Mouse_PlayerController_C|GetHUD%20Reference _asbp_mouse_player_controller) self))

(fn ConstructionScript)

(fn TowerShoot)

(fn LevelUp)