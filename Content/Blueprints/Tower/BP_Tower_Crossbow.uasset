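; Crossbow tower Blueprint that shoots projectiles at a target and can be upgraded, built on a parent tower class.
; While a target is in range, Tick turns the crossbow toward it using a yaw-only look-at with an offset.
; Shooting spawns a BP_Projectile at the crossbow, passing it target and damage.
; Leveling up shortens reload, raises damage, plays effects and swaps the stone tower mesh by level.
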(event EventTick
  (params (DeltaSeconds :type Float%20%28single-precision%29))
  (bind (_returnvalue _crossbow) (|RotateTowardTarget))
  (if (Variables|Default|GetisInRange)
    (Transformation|SetWorldRotation _crossbow _returnvalue false)))

(event EventLevelUp
  (CallFunction|LevelUpCrossbow))

(event EventTowerShoot
  (CallFunction|CrossbowShoot))

(fn ConstructionScript
  (|CallParentFunction)
  (Variables|Default|SetProjectile "/Game/Blueprints/Tower/BP_Projectile.BP_Projectile_C"))

(fn CrossbowShoot
  (bind _returnvalue (Game|SpawnActorfromClass (Variables|Default|GetProjectile) (Transformation|GetWorldTransform (Variables|Default|GetCrossbow)) false 0))
  (bind _asbp_projectile (Utilities|Casting|CastToBP_Projectile _returnvalue))
  (Variables|/Game/Blueprints/Tower/BP_Projectile.BP_Projectile_C|SetTarget _asbp_projectile (Variables|Default|GetTarget))
  (Variables|/Game/Blueprints/Tower/BP_Projectile.BP_Projectile_C|SetDamage _asbp_projectile (Variables|Default|GetProjectileDamage))
  (Audio|PlaySoundatLocation "/Game/Sound/S_CrossbowShot.S_CrossbowShot" (Transformation|GetActorLocation _returnvalue)))

(fn LevelUpCrossbow
  (bind _tower_attack_area (Variables|Default|GetTower_Attack_Area))
  (bind _returnvalue (Transformation|GetWorldLocation _tower_attack_area))
  (Variables|Default|SetReloadTime (- (Variables|Default|GetReloadTime) 0.375))
  (Variables|Default|SetProjectileDamage (+ (Variables|Default|GetProjectileDamage) 0.25))
  (Variables|Default|SetLevel (+ (Variables|Default|GetLevel) 1))
  (Effects|SpawnEmitteratLocation "/Game/Particles/P_LevelUp.P_LevelUp" _returnvalue)
  (Audio|PlaySoundatLocation "/Game/Sound/S_LevelUp.S_LevelUp" _returnvalue)
  (if (== (Variables|Default|GetLevel) 1)
    (Components|StaticMesh|SetStaticMesh "/Game/Meshes/StoneTower.StoneTower")
    (else
      (Components|StaticMesh|SetStaticMesh "/Game/Meshes/ProtectedStoneTower.ProtectedStoneTower"))))