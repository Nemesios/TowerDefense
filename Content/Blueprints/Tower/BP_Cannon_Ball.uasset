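; Homing cannonball projectile for a tower, which chases its Target and explodes with radial damage.
; Each Tick moves the construction-script-created CanonBall mesh toward the target at Speed and rotates it to face it.
; Overlapping the target applies configurable area damage with explosion effect and sound, then destroys the actor.
; If the target is invalid, it applies fixed radial damage near the ball, exploding and self-destroying only when that damage lands.
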(event OnComponentBeginOverlap(CanonBall)
  (params (OtherActor :type Actor%20Object%20Reference) (OtherComp :type Primitive%20Component%20Object%20Reference) (OtherBodyIndex :type Integer) (bFromSweep :type Boolean) (SweepResult :type Hit%20Result%20Structure%20%28by%20ref%29))
  (bind _target (Variables|Default|GetTarget))
  (if (== OtherActor _target)
    (bind _returnvalue (Effects|SpawnEmitteratLocation "/Game/StarterContent/Particles/P_Explosion.P_Explosion" (Transformation|GetActorLocation _target)))
    (Game|Damage|ApplyRadialDamage (Variables|Default|GetDamage) (Transformation|GetWorldLocation _returnvalue) (Variables|Default|GetDamageRadius) "/Script/Engine.DamageType" 0 self 0 true "ECC_Visibility")
    (Audio|PlaySoundatLocation "/Game/StarterContent/Audio/Explosion01.Explosion01" (Transformation|GetWorldLocation _returnvalue))
    (Actor|DestroyActor)))

(event EventTick
  (params (DeltaSeconds :type Float%20%28single-precision%29))
  (bind _target (Variables|Default|GetTarget))
  (bind _canonball (Variables|Default|GetCanonBall))
  (bind _canonball_2 (Variables|Default|GetCanonBall))
  (bind _returnvalue (Transformation|GetActorLocation _target))
  (bind _returnvalue_2 (Transformation|GetWorldLocation _canonball))
  (bind _returnvalue_3 (Transformation|GetWorldLocation _canonball_2))
  (bind _returnvalue_4 (Math|Rotator|FindLookatRotation _returnvalue_2 _returnvalue))
  (bind (_x _y) (Math|Vector|BreakVector _returnvalue_3))
  (bind (_pitch _yaw) (Class|KismetMathLibrary|BreakRot _returnvalue_4))
  (bind _returnvalue_5 (+ _x 7e+01))
  (bind _returnvalue_6 (+ _y 7e+01))
  (bind _returnvalue_7 (Math|Vector|MakeVector _returnvalue_5 _returnvalue_6 2e+01))
  ;[1 1 1] Set new location every frame
  (if (Utilities|IsValid (Variables|Default|GetTarget))
    (Transformation|SetWorldTransform (Variables|Default|GetCanonBall) (Math|Transform|MakeTransform (+ (* (Math|Vector|Normalize (- (Transformation|GetActorLocation (Variables|Default|GetTarget)) (Transformation|GetWorldLocation (Variables|Default|GetCanonBall)))) (* (Utilities|Time|GetWorldDeltaSeconds) (Variables|Default|GetSpeed))) (Transformation|GetWorldLocation (Variables|Default|GetCanonBall))) (Class|KismetMathLibrary|MakeRot (+ _pitch -9e+01) (+ _yaw -9e+01) 0.0)) false)
    (else
      (bind _returnvalue_8 (Game|Damage|ApplyRadialDamage 5.0 _returnvalue_7 3e+02 0 0 0 0 false "ECC_Visibility"))
      (if _returnvalue_8
        (Effects|SpawnEmitteratLocation "/Game/StarterContent/Particles/P_Explosion.P_Explosion" _returnvalue_7)
        (Audio|PlaySoundatLocation "/Game/StarterContent/Audio/Explosion01.Explosion01" _returnvalue_7)
        (Actor|DestroyActor)))))

(fn ConstructionScript
  (bind _returnvalue (AddComponent|AddStaticMeshComponent false))
  (Variables|Default|SetCanonBall _returnvalue))