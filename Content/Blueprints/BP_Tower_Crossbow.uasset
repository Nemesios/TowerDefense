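; BP_Tower_Crossbow is a crossbow tower that turns toward and fires projectiles at a target.
; While a target is in range, Tick rotates the Crossbow component using RotateTowardTarget.
; The TowerShoot event calls CrossbowShoot, which spawns a BP_Projectile at the crossbow's transform and passes it the Target and damage.
; LevelUp shortens reload time, raises projectile damage and increments the level by fixed steps.
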(event EventTick
  (params (DeltaSeconds :type Float%20%28single-precision%29))
  (bind (_returnvalue _crossbow) (|RotateTowardTarget))
  (if (Variables|Default|GetisInRange)
    (Transformation|SetWorldRotation _crossbow _returnvalue false)))

(event EventTowerShoot
  (CallFunction|CrossbowShoot))

(fn ConstructionScript
  (|CallParentFunction)
  (Variables|Default|SetProjectile "/Game/Blueprints/BP_Projectile.BP_Projectile_C"))

(fn CrossbowShoot
  (bind _returnvalue (Game|SpawnActorfromClass (Variables|Default|GetProjectile) (Transformation|GetWorldTransform (Variables|Default|GetCrossbow)) false 0))
  (bind _asbp_projectile (Utilities|Casting|CastToBP_Projectile _returnvalue))
  (Variables|/Game/Blueprints/BP_Projectile.BP_Projectile_C|SetTarget _asbp_projectile (Variables|Default|GetTarget))
  (Variables|/Game/Blueprints/BP_Projectile.BP_Projectile_C|SetDamage _asbp_projectile (Variables|Default|GetProjectileDamage)))

(fn LevelUp
  (Variables|Default|SetReloadTime (- (Variables|Default|GetReloadTime) 0.375))
  (Variables|Default|SetProjectileDamage (+ (Variables|Default|GetProjectileDamage) 0.25))
  (Variables|Default|SetLevel (+ (Variables|Default|GetLevel) 1)))