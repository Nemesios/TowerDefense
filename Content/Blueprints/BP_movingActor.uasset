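; BP_movingActor is a damageable actor that moves in a straight line along its Direction until destroyed.
; Each Tick sets the actor transform from the Enemy component's world transform, offset by normalized Direction times Speed and delta time, without sweeping.
; AnyDamage subtracts floored damage from Health and destroys the actor at zero or below, with damage enabled in the construction script.
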(event EventAnyDamage
  (params (Damage :type Float%20%28single-precision%29) (DamageType :type Damage%20Type%20Object%20Reference) (InstigatedBy :type Controller%20Object%20Reference) (DamageCauser :type Actor%20Object%20Reference))
  (Variables|Default|Sethealth (- (Variables|Default|Gethealth) (Math|Float|Floor Damage)))
  (Math|Integer|CompareInt (Variables|Default|Gethealth) 0
    (:==
      _)
    (:<
      _))
  (Actor|DestroyActor))

(event EventTick
  (params (DeltaSeconds :type Float%20%28single-precision%29))
  (bind _enemy (Variables|Default|Getenemy))
  (bind _returnvalue (Transformation|GetWorldTransform _enemy))
  (bind (_location _rotation _scale) (Math|Transform|BreakTransform _returnvalue))
  (Transformation|SetActorTransform (Math|Transform|MakeTransform (+ (* (Math|Vector|Normalize (Variables|Default|GetDirection)) (* (Utilities|Time|GetWorldDeltaSeconds) (Variables|Default|GetSpeed))) _location) _rotation _scale)))

(fn ConstructionScript
  (Variables|Actor|SetbCanBeDamaged true))