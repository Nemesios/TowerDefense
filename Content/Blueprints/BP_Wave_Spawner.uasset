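; BP_Wave_Spawner spawns configured waves of enemies at its own location, handing each enemy the wave's spline data and the mouse player controller.
; CustomStart schedules CustomLaunchNextWave after a one-shot delay, which selects the next wave and starts a looping spawn timer at that wave's interval.
; Each tick spawns and records one enemy until the list ends.
; CustomStop cancels pending launches and records whether waves completed.
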(event Custom|Custom%20Start
  (if (> (Utilities|Array|Length (Variables|Default|GetWaves)) 0)
    (if (not (Variables|Default|GetHasStarted))
      (Variables|Default|SetHasStarted (== (Variables|Default|GetWaveIndex) 0))
      (Utilities|Time|SetTimerbyFunctionName self "Custom LaunchNextWave" (Variables|Default|GetTimeBetweenWaves)))
    (else
      (Development|PrintString "No Wave Set"))))

(event Custom|Custom%20Stop
  (params (Waves%20Completed :type Boolean))
  (if (Variables|Default|GetHasStarted)
    (Utilities|Time|ClearTimerbyFunctionName self "Custom LaunchNextWave")
    (Variables|Default|SetHasStarted false)
    (Variables|Default|SetWavesCompleted Waves%20Completed)))

(event Custom|Custom%20LaunchNextWave
  (if (< (Variables|Default|GetWaveIndex) (Utilities|Array|Length (Variables|Default|GetWaves)))
    (Variables|Default|SetActualWave (Utilities|Array|Get(acopy) (Variables|Default|GetWaves) (Variables|Default|GetWaveIndex)))
    (Utilities|Time|SetTimerbyFunctionName 0 "Custom SpawnEnemy" (.Intervale (Utilities|Struct|BreakS_Wave (Utilities|Array|Get(acopy) (Variables|Default|GetWaves) (Variables|Default|GetWaveIndex)))) true)
    (Variables|Default|SetWaveIndex (+ (Variables|Default|GetWaveIndex) 1))
    (else
      (CallFunction|CustomStop true))))

(event Custom|Custom%20SpawnEnemy
  (bind _actualwave (Variables|Default|GetActualWave))
  (bind (_enemies _splines) (Utilities|Struct|BreakS_Wave _actualwave))
  (if (< (Variables|Default|GetEnemyIndex) (Utilities|Array|Length (.Enemies (Utilities|Struct|BreakS_Wave (Variables|Default|GetActualWave)))))
    (bind _returnvalue (Game|SpawnActorfromClass (Utilities|Array|Get(acopy) _enemies (Variables|Default|GetEnemyIndex)) (Math|Transform|MakeTransform (Transformation|GetActorLocation self)) true _splines 0))
    (Utilities|Array|Add (Variables|Default|GetEnemiesSpawned) _returnvalue)
    (Variables|/Game/Characters/BP_Enemy_Master.BP_Enemy_Master_C|SetPlayerController _returnvalue (Variables|Default|GetPlayerController))
    (Variables|Default|SetEnemyIndex (+ (Variables|Default|GetEnemyIndex) 1))
    (else
      (Utilities|Time|ClearTimerbyFunctionName 0 "Custom SpawnEnemy")
      (Variables|Default|SetEnemyIndex 0))))

(event EventBeginPlay
  (bind _asbp_mouse_player_controller (Utilities|Casting|CastToBP_Mouse_PlayerController (Game|GetPlayerController 0)))
  (Variables|Default|SetPlayerController _asbp_mouse_player_controller))

(fn ConstructionScript)